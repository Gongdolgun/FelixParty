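; Lobby player controller that shows the lobby screen and keeps its player list current.
; On BeginPlay it enables the mouse cursor and uses an authority switch to add either the host or client lobby widget to the viewport.
; Player list updates are stored, then after a short delay passed to whichever widget matches the controller's authority.
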(event `self.ReceiveBeginPlay`
  (`self.CreateMenus`)
  (set `self.bShowMouseCursor` true))

(event `CreateMenus`
  ;[1 1 1] Create Menu Widget
  (`/Engine/EditorBlueprintResources/ActorMacros.Switch Has Authority`
    (:`Authority`
      (bind _returnvalue (`|CreateWidget` "/Game/Widgets/Session/WDG_LobbyHostScreen.WDG_LobbyHostScreen_C"))
      (bind _output_get (set `self.LobbyWidget` _returnvalue))
      (`UserWidget.AddToViewport` _output_get 0))
    (:`Remote`
      (bind _returnvalue_2 (`|CreateWidget` "/Game/Widgets/Session/WDG_LobbyClientScreen.WDG_LobbyClientScreen_C"))
      (bind _output_get_2 (set `self.LobbyWidget` _returnvalue_2))
      (`UserWidget.AddToViewport` _output_get_2 0))))

(event `self.UpdatePlayerList`
  (params (PlayerBaseInfos :type "Array of PlayerBaseInfo Structure (by ref)"))
  ;[1 1 1] NativeEvent
  (`self.UpdateList` PlayerBaseInfos))

(event `UpdateList`
  (params (`Player Infos` :type "Array of PlayerBaseInfo Structure"))
  (bind _playerinfos (`self.PlayerInfos`))
  ;[1 1 1] NativeEvent
  (set `self.PlayerInfos` `Player Infos`)
  (`KismetSystemLibrary.Delay` 0.2)
  (`/Engine/EditorBlueprintResources/ActorMacros.Switch Has Authority`
    (:`Authority`
      (bind _aswdg_lobby_host_screen (cast `/Game/Widgets/Session/WDG_LobbyHostScreen` (`self.LobbyWidget`)))
      (`LobbyScreen.UpdatePlayerList` _aswdg_lobby_host_screen _playerinfos))
    (:`Remote`
      (bind _aswdg_lobby_client_screen (cast `/Game/Widgets/Session/WDG_LobbyClientScreen` (`self.LobbyWidget`)))
      (`LobbyScreen.UpdatePlayerList` _aswdg_lobby_client_screen _playerinfos))))

(fn `UserConstructionScript`)