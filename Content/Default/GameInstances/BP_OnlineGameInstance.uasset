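; Game instance that handles online session hosting, joining and invites, and persists player settings.
; Hosting creates an Advanced Sessions session with a custom name, then opens the Lobby as a listen server; failures create an error widget.
; Received invites display an invite card carrying the session, and accepted invites join it.
; Settings are cached on the instance and saved to or loaded from an SG_SaveSettings slot.
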(event `HostSession`
  (params (`Number Of Player` :type Integer) (SessionName :type String) (`Use LAN` :type Boolean))
  ;[1 1 1] Hosting and Joining Session
  (bind _output_get (set `self.Number Of Player` `Number Of Player`))
  (`CreateSessionCallbackProxyAdvanced.CreateAdvancedSession` (`|MakeArray` (`AdvancedSessionsLibrary.MakeLiteralSessionPropertyString` "SessionName" SessionName)) (`GameplayStatics.GetPlayerController` 0) _output_get 0 `Use LAN`
    (:`OnSuccess`
      (`AsyncLoadingScreenLibrary.SetDisplayBackgroundIndex` 0)
      (`AsyncLoadingScreenLibrary.SetDisplayTipTextIndex` 0)
      (`GameplayStatics.OpenLevelBySoftObjectPtr` "/Game/Levels/Lobby.Lobby" true "?listen"))
    (:`OnFailure`
      (`|CreateWidget` "/Game/Widgets/Session/WDG_ErrorMessage.WDG_ErrorMessage_C" null "Failed to create a session. Please Check network connection."))))

(event `JoinSession`
  (params (Session :type "BlueprintSessionResult Structure"))
  (bind _returnvalue (`GameplayStatics.GetPlayerController` 0))
  ;[1 1 1] Hosting and Joining Session
  (`JoinSessionCallbackProxy.JoinSession` _returnvalue Session
    (:`OnFailure`
      (`|CreateWidget` "/Game/Widgets/Session/WDG_ErrorMessage.WDG_ErrorMessage_C" _returnvalue "Failed to create a session. Please Check network connection."))))

(event `self.OnSessionInviteAccepted`
  (params (LocalPlayerNum :type Integer) (PersonInvited :type "BPUniqueNetId Structure") (SessionToJoin :type "BlueprintSessionResult Structure (by ref)"))
  (bind _returnvalue (`GameplayStatics.GetPlayerController` 0))
  ;[1 1 1] Hosting and Joining Session
  (`JoinSessionCallbackProxy.JoinSession` _returnvalue SessionToJoin
    (:`OnFailure`
      (`|CreateWidget` "/Game/Widgets/Session/WDG_ErrorMessage.WDG_ErrorMessage_C" _returnvalue "Failed to create a session. Please Check network connection."))))

(event `self.OnSessionInviteReceived`
  (params (LocalPlayerNum :type Integer) (PersonInviting :type "BPUniqueNetId Structure") (AppId :type String) (SessionToJoin :type "BlueprintSessionResult Structure (by ref)"))
  ;[1 1 1] Hosting and Joining Session
  (`KismetSystemLibrary.PrintString` "Invitation  Accepted")
  (bind _returnvalue (`|CreateWidget` "/Game/Widgets/Session/Invitation/WDG_InviteCard.WDG_InviteCard_C" (`GameplayStatics.GetPlayerController` 0) (`KismetStringLibrary.Concat_StrStr` (`AdvancedIdentityLibrary.GetPlayerNickname` PersonInviting) " 님이 세션에 초대했습니다. 수락 하시겠습니까?") SessionToJoin))
  (`UserWidget.AddToViewport` _returnvalue 0))

(event `/Game/Default/SaveSetting/I_SettingsManager.SaveSettings`
  (params (`In Settings` :type "SaveSettings Structure"))
  (set `self.Instance_Settings` `In Settings`)
  (bind _returnvalue (`self.Get Save`))
  (set `DefualtSaveGame.SaveSettings` (`self.Instance_Settings`) _returnvalue)
  (`GameplayStatics.SaveGameToSlot` _returnvalue (`self.SettingsSlotSave`)))

(event `/Game/Default/SaveSetting/I_SettingsManager.LoadSettings`
  (bind _returnvalue (`GameplayStatics.DoesSaveGameExist` (`self.SettingsSlotSave`)))
  (if _returnvalue
    (bind _returnvalue_2 (`GameplayStatics.LoadGameFromSlot` (`self.SettingsSlotSave`)))
    (bind _assg_save_settings (cast `/Game/Default/SaveSetting/SG_SaveSettings` _returnvalue_2))
    (set `self.Instance_Settings` (`DefualtSaveGame.SaveSettings` _assg_save_settings))))

(fn `Get Save`
  (returns (ReturnValue :type "/Game/Default/SaveSetting/SG_SaveSettings Object Reference"))
  (bind _returnvalue (`GameplayStatics.DoesSaveGameExist` (`self.SettingsSlotSave`)))
  (if _returnvalue
    (bind _returnvalue_2 (`GameplayStatics.LoadGameFromSlot` (`self.SettingsSlotSave`)))
    (bind _assg_save_settings (cast `/Game/Default/SaveSetting/SG_SaveSettings` _returnvalue_2))
    (return _assg_save_settings)
    (else
      (bind _returnvalue_3 (`GameplayStatics.CreateSaveGameObject` "/Game/Default/SaveSetting/SG_SaveSettings.SG_SaveSettings_C"))
      (return _returnvalue_3))))