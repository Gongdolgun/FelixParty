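; Lobby game mode that shows each connected player as a spawned character on a lobby platform.
; On BeginPlay it gathers BP_LobbyPlatForm actors, ordered by tags matching their index.
; Login and logout update the player controller list, then a macro polls until platform setup finishes.
; The update pass assigns unplaced players to the first free platform and clears platforms whose player has left.
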(event `self.ReceiveBeginPlay`
  (`parent.ReceiveBeginPlay`)
  (`self.SetUpPlatforms`))

(event `self.K2_PostLogin`
  (params (NewPlayer :type "PlayerController Object Reference"))
  (`parent.K2_PostLogin` NewPlayer)
  (`KismetArrayLibrary.Array_Add` (`self.PCs`) NewPlayer)
  (`self.IfPlatformsSetUpIsDone` :!label _label
    (:`True`
      (`self.UpdatePlayersOnPlatforms`))))

(event `self.K2_OnLogout`
  (params (ExitingController :type "Controller Object Reference"))
  (`parent.K2_OnLogout` ExitingController)
  (bind `_as플레이어_컨트롤러` (cast `PlayerController` ExitingController))
  (`KismetArrayLibrary.Array_RemoveItem` (`self.PCs`) `_as플레이어_컨트롤러`)
  (goto _label))

(fn `SetUpPlatforms`
  (bind _outactors (`GameplayStatics.GetAllActorsOfClass` "/Game/GameTypes/OnlyUp/Actors/BP_LobbyPlatForm.BP_LobbyPlatForm_C"))
  (for _index (range (+ (`KismetArrayLibrary.Array_LastIndex` _outactors) 1))
    (bind _outactors_2 (`GameplayStatics.GetAllActorsOfClassWithTag` "/Game/GameTypes/OnlyUp/Actors/BP_LobbyPlatForm.BP_LobbyPlatForm_C" (`KismetStringLibrary.Conv_StringToName` (`KismetStringLibrary.Conv_IntToString` _index))))
    (`KismetArrayLibrary.Array_Add` (`self.LobbyPlatforms`) (`|GetArrayItem` _outactors_2)))
  (set `self.bPlatformSetUpDone` true))

(fn `UpdatePlayersOnPlatforms`
  (locals (LoopPCAllReadyAdded :type Boolean))
  (for _array_element (`self.PCs`)
    (set `local.LoopPCAllReadyAdded` false)
    (for _array_element_2 (`self.LobbyPlatforms`)
      (if (== (`/Game/GameTypes/OnlyUp/Actors/BP_LobbyPlatForm.PlayerController` _array_element_2) _array_element)
        (set `local.LoopPCAllReadyAdded` true)
        (break)))
    (if (not (`local.LoopPCAllReadyAdded`))
      (for _array_element_3 (`self.LobbyPlatforms`)
        (`/Engine/EditorBlueprintResources/StandardMacros.IsValid` (`/Game/GameTypes/OnlyUp/Actors/BP_LobbyPlatForm.PlayerController` _array_element_3)
          (:`Is Not Valid`
            (`/Game/GameTypes/OnlyUp/Actors/BP_LobbyPlatForm.SpawnCharacter` _array_element_3 _array_element)
            (break))))))
  (for _array_element_4 (`self.LobbyPlatforms`)
    (if (not (`KismetArrayLibrary.Array_Contains` (`self.PCs`) (`/Game/GameTypes/OnlyUp/Actors/BP_LobbyPlatForm.PlayerController` _array_element_4)))
      (`/Game/GameTypes/OnlyUp/Actors/BP_LobbyPlatForm.Clear` _array_element_4))))

(fn `UserConstructionScript`)