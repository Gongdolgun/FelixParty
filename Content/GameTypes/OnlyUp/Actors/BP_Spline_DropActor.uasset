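; Only Up actor that travels along a linked spline when a character touches it, then drops and respawns.
; Box overlap sets the character's SpawnIndex and starts the move through server and NMC events, with a timeline interpolating distance along the spline.
; At the end the cube gets physics and a downward impulse, then a timer spawns a replacement at the initial location with the same spline and destroys this actor.
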(event `self.ReceiveBeginPlay`
  (set `self.InitLocation` (`self.K2_GetActorLocation`))
  (set `self.TempSplineComponent` (`self.SplineComponent`)))

(event `MoveObject_Server`
  (`self.MoveObject_NMC`))

(event `MoveObject_NMC`
  (`TimelineComponent.SetPlayRate` (`self.MoveObject T`) (/ 1.0 (`self.TimeToComplete`)))
  (bind (_direction `_새_트랙_0`) (`Timeline|MoveObject T` :!via `PlayFromStart`)
    (:`Update`
      (`self.K2_SetActorTransform` (`KismetMathLibrary.MakeTransform` (`SplineComponent.GetLocationAtDistanceAlongSpline` (`/Game/GameTypes/OnlyUp/Actors/BP_SplineMovement.Spline` (`self.SplineComponent`)) (`KismetMathLibrary.Lerp` 0.0 (`SplineComponent.GetSplineLength` (`/Game/GameTypes/OnlyUp/Actors/BP_SplineMovement.Spline` (`self.SplineComponent`))) `_새_트랙_0`) "World") (struct) (`self.GetActorScale3D`))))
    (:`Finished`
      (`self.SettingDrops`))))

(event `SettingDrops`
  (bind _cube (`self.Cube`))
  (`PrimitiveComponent.SetSimulatePhysics` _cube true)
  (`PrimitiveComponent.AddImpulse` _cube (0.0 0.0 -100.0) "None" false)
  (`KismetSystemLibrary.K2_SetTimerDelegate` (delegate `Set Init Location`) 3.0))

(event `Set Init Location`
  (bind _returnvalue (`|SpawnActorFromClass` (`GameplayStatics.GetObjectClass` self) (`KismetMathLibrary.Conv_VectorToTransform` (`self.InitLocation`)) "AlwaysSpawn" "MultiplyWithRoot" null null))
  (set `/Game/GameTypes/OnlyUp/Actors/BP_Spline_DropActor.SplineComponent` (`self.TempSplineComponent`) _returnvalue)
  (`self.K2_DestroyActor`))

(event `self.Box.OnComponentBeginOverlap`
  (params (OverlappedComponent :type "PrimitiveComponent Object Reference") (OtherActor :type "Actor Object Reference") (OtherComp :type "PrimitiveComponent Object Reference") (OtherBodyIndex :type Integer) (bFromSweep :type Boolean) (SweepResult :type "HitResult Structure (by ref)"))
  (if (!= self OtherActor)
    (bind _asonly_up_character (cast `OnlyUpCharacter` OtherActor))
    (bind _output_get (set `self.As Only Up Character` _asonly_up_character))
    (`/Engine/EditorBlueprintResources/StandardMacros.IsValid` (`self.SplineComponent`)
      (:`Is Valid`
        (`self.MoveObject_Server`)
        (set `OnlyUpCharacter.SpawnIndex` 2 _output_get)))))

(fn `UserConstructionScript`
  (bind _splinecomponent (`self.SplineComponent`))
  (`/Engine/EditorBlueprintResources/StandardMacros.IsValid` _splinecomponent
    (:`Is Valid`
      (`self.K2_SetActorLocation` (`SplineComponent.GetLocationAtSplinePoint` (`/Game/GameTypes/OnlyUp/Actors/BP_SplineMovement.Spline` _splinecomponent) 0 "World")))))