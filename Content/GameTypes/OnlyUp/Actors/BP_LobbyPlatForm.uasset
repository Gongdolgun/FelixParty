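; BP_LobbyPlatForm is an Only Up lobby platform actor meant to show a player's character at a marked spawn point.
; Its graph holds logic to clear the player controller and destroy the current character, or replace it with a new BP_LobbyCharacter.
; The new character spawns at PlayerSpawnTransform with a small offset, mostly upward.
; Neither chain is wired to run, and the construction script is empty.
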(fn `UserConstructionScript`)