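; Spline-following actor for the OnlyUp game type that travels repeatedly along the spline of a referenced spline object.
; The construction script snaps it to the first spline point, and BeginPlay starts movement through a server-to-multicast event pair.
; A timeline, rate-scaled by TimeToComplete, lerps distance along the spline to set location, leaving spline rotation unused.
; On finish, a timer restarts the run from the beginning after RestartTime.
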(event `self.ReceiveBeginPlay`
  (`/Engine/EditorBlueprintResources/StandardMacros.IsValid` (`self.SplineComponent`)
    (:`Is Valid`
      (`self.MoveObject_Server`))))

(event `MoveObject_Server`
  (`self.MoveObject_NMC`))

(event `MoveObject_NMC`
  (`TimelineComponent.SetPlayRate` (`self.MoveObject T`) (/ 1.0 (`self.TimeToComplete`)))
  (bind (_direction `_새_트랙_0`) (`Timeline|MoveObject T` :!via `PlayFromStart`)
    (:`Update`
      (`self.K2_SetActorTransform` (`KismetMathLibrary.MakeTransform` (`SplineComponent.GetLocationAtDistanceAlongSpline` (`/Game/GameTypes/OnlyUp/Actors/BP_SplineMovement.Spline` (`self.SplineComponent`)) (`KismetMathLibrary.Lerp` 0.0 (`SplineComponent.GetSplineLength` (`/Game/GameTypes/OnlyUp/Actors/BP_SplineMovement.Spline` (`self.SplineComponent`))) `_새_트랙_0`) "World") (struct) (`self.GetActorScale3D`))))
    (:`Finished`
      (`KismetSystemLibrary.K2_SetTimerDelegate` (delegate `MoveObject_Server`) (`self.RestartTime`)))))

(fn `UserConstructionScript`
  (`self.K2_SetActorLocation` (`SplineComponent.GetLocationAtSplinePoint` (`/Game/GameTypes/OnlyUp/Actors/BP_SplineMovement.Spline` (`self.SplineComponent`)) 0 "World")))