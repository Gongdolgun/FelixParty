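; Only Up player character that mantles obstacles ahead, or jumps when no parkour is possible.
; V uses a Blueprint line-and-sphere trace to find two ledge points, with reduced reach while falling; Space uses ParkourComponent's equivalent trace.
; M_Parkour feeds both points to Motion Warping and plays the component's montage, disabling collision in Flying mode until a timed delay restores collision and sets Falling.
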(event `Key|V`
  (params (Key :type "Key Structure"))
  (:`Pressed`
    (bind (_inparkourpos1 _inparkourpso2) (`self.Parkour Trace BP` 50.0 120.0 0.5 "ForDuration"))
    (if (`self.CanParkour`)
      (`self.M_Parkour` _inparkourpos1 _inparkourpso2 -45.0 -10.0 1.0)
      (else
        (`self.Jump`)))))

(event `Key|SpaceBar`
  (params (Key :type "Key Structure"))
  (bind _parkourcomponent (`self.ParkourComponent`))
  (:`Pressed`
    (`ParkourComponent.ParkourTrace` :`self` _parkourcomponent :`InInitialTraceLength` 50.0 :`InSecondaryTraceZOffset` 120.0 :`InFallingHeightMultiplier` 0.5)
    (if (`ParkourComponent.bCanParkour` _parkourcomponent)
      (`self.M_Parkour` (`ParkourComponent.GetParkourPos1` _parkourcomponent) (`ParkourComponent.GetParkourPos2` _parkourcomponent) -35.0 -10.0 1.1)
      (else
        (`self.Jump`)))))

(fn `Parkour Trace BP`
  (params (Initial_Trace_Length :type "Float (double-precision)") (Trace_Z_Offset :type "Float (double-precision)") (Falling_Height_Multiplier :type "Float (double-precision)") (DebugTrace :type "EDrawDebugTrace Enum" :default "None"))
  (returns (InParkourPos1 :type "Vector Structure") (InParkourPso2 :type "Vector Structure"))
  (locals (MantlePos1 :type "Vector Structure") (MantlePos2 :type "Vector Structure"))
  (bind _returnvalue (`self.K2_GetActorLocation`))
  (bind (_mantlepos1_x _mantlepos1_y) (`KismetMathLibrary.BreakVector` (`local.MantlePos1`)))
  (bind _returnvalue_2 (+ (`local.MantlePos2`) (0.0 0.0 100.0)))
  ;[1 1 1] Trace to Check for an Obejct
  (set `self.CanParkour` false)
  (bind (_outhit _returnvalue_3) (`KismetSystemLibrary.LineTraceSingle` :`Start` _returnvalue :`End` (+ _returnvalue (* (`self.GetActorForwardVector`) Initial_Trace_Length)) :`TraceChannel` "TraceTypeQuery1" :`DrawDebugType` (`local.DebugTrace`)))
  ;[1 1 1] Object가 발견되면 Object 높이를 추적합니다. Player가 Falling이면 최대 도달 가능 높이가 낮아집니다
  (if _returnvalue_3
    (bind (_bblockinghit _binitialoverlap _time _distance _location) (`GameplayStatics.BreakHitResult` _outhit))
    (bind (_outhit_2 _returnvalue_4) (`KismetSystemLibrary.SphereTraceSingle` :`Start` (+ _location (`KismetMathLibrary.MakeVector` 0.0 0.0 (* (`local.Trace_Z_Offset`) (`KismetMathLibrary.SelectFloat` (`local.Falling_Height_Multiplier`) 1.0 (`NavMovementComponent.IsFalling` (`self.CharacterMovement`)))))) :`End` _location :`Radius` 10.0 :`TraceChannel` "TraceTypeQuery1" :`DrawDebugType` (`local.DebugTrace`)))
    ;[1 1 1] 추적에서 검출된 점을 사용하여 이동 워프할 위치 찾기
    (if _returnvalue_4
      (bind (_bblockinghit_2 _binitialoverlap_2 _time_2 _distance_2 _location_2 _impactpoint) (`GameplayStatics.BreakHitResult` _outhit_2))
      (set `local.MantlePos1` (+ _impactpoint (* (`self.GetActorForwardVector`) -50.0)))
      (bind _output_get (set `local.MantlePos2` (+ _impactpoint (* (`self.GetActorForwardVector`) 120.0))))
      ;[1 1 1] 이것은 두 번째 모션 워프 위치를 추론합니다.
      (set `self.CanParkour` true)
      (bind _returnvalue_5 (+ _output_get (0.0 0.0 20.0)))
      (bind (_outhit_3 _returnvalue_6) (`KismetSystemLibrary.SphereTraceSingle` :`Start` _returnvalue_5 :`End` _returnvalue_5 :`Radius` 10.0 :`TraceChannel` "TraceTypeQuery1" :`DrawDebugType` (`local.DebugTrace`)))
      (if _returnvalue_6
        (set `self.CanParkour` false)
        (else
          (set `local.MantlePos2` (+ _impactpoint (* (`self.GetActorForwardVector`) 50.0)))))
      ;[1 1 1] 첫 번째와 두 번째 맨틀 위치의 경로가 명확한지 확인하기 위해 마지막 추적을 수행
      (if (or (== (`local.MantlePos1`) (0.0 0.0 0.0)) (== (`local.MantlePos2`) (0.0 0.0 0.0)))
        (set `self.CanParkour` false :!label _label)
        (else
          (bind (_outhit_4 _returnvalue_7) (`KismetSystemLibrary.SphereTraceSingle` :`Start` (`KismetMathLibrary.MakeVector` _mantlepos1_x _mantlepos1_y (.z _returnvalue_2)) :`End` _returnvalue_2 :`Radius` 10.0 :`TraceChannel` "TraceTypeQuery1" :`DrawDebugType` (`local.DebugTrace`)))
          (if _returnvalue_7
            (goto _label)
            (else
              _))))
      (return (`local.MantlePos1`) (`local.MantlePos2`)))
    (else
      (set `self.CanParkour` false))))

(fn `UserConstructionScript`)

(fn `새 함수`)