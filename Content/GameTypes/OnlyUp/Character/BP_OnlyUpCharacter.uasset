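; Player character for the OnlyUp game mode that turns Space into a context parkour move or a normal jump.
; ParkourComponent traces and supplies per-type settings; when it allows parkour and StateComponent is idle, the move runs in flying mode without collision, with a montage and slowed camera lag.
; Server-to-multicast events set motion warp targets, both named ParkourPoint1.
; Also holds a Blueprint ledge trace and an input-locked spawn material fade.
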(event `self.ReceiveBeginPlay`
  (`parent.ReceiveBeginPlay`)
  (bind _asbp_only_up_game_state (cast `/Game/GameTypes/OnlyUp/GameState/BP_OnlyUpGameState` (`GameplayStatics.GetGameState`)))
  (set `self.As BP Only Up Game State` _asbp_only_up_game_state))

(event `self.PlayerMaterialEventOnSpawn`
  (`self.PlayMaterialEvent_NMC`))

(event `PlayMaterialEvent_NMC`
  (`self.DisableInput` (`GameplayStatics.GetPlayerController` 0))
  (bind (_direction `_새_트랙_0`) (`Timeline|타임라인` :!via `PlayFromStart`)
    (:`Update`
      (for _array_element (`self.MyMaterials`)
        (`MaterialInstanceDynamic.SetScalarParameterValue` _array_element "Appearance" `_새_트랙_0`)))
    (:`Finished`
      (`self.EnableInput` (`GameplayStatics.GetPlayerController` 0)))))

(event `Key|SpaceBar`
  (params (Key :type "Key Structure"))
  (bind _parkourcomponent (`self.ParkourComponent`))
  (bind _parkourcomponent_2 (`self.ParkourComponent`))
  (bind _returnvalue (`StateComponent.GetCurrState` (`self.StateComponent`)))
  (bind ((`OutLocation1` _outlocation1) (`OutLocation2` _outlocation2) (`ParkourType` _parkourtype)) (break `ParkourStruct` (`ParkourComponent.OutParkourStruct` (`self.ParkourComponent`))))
  ;[1 1 1] Parkour
  (:`Pressed`
    (`ParkourComponent.ParkourTrace` (`self.ParkourComponent`) (`ParkourComponent.OutParkourStruct` _parkourcomponent) (`ParkourComponent.Initial_Trace_Length` _parkourcomponent) (`ParkourComponent.Trace_Z_Offset` _parkourcomponent) (`ParkourComponent.Falling_Height_Multiplier` _parkourcomponent))
    (if (and (`ParkourComponent.bCanParkour` (`self.ParkourComponent`)) (`|EnumEquality` _returnvalue "Idle"))
      (`StateComponent.SetActionMode` (`self.StateComponent`))
      (`KismetSystemLibrary.PrintString` (`|GetEnumeratorNameAsString` _returnvalue))
      (switch `EParkourType` _parkourtype
        (:`High`
          (set `ParkourComponent.ResultStruct` (`ParkourComponent.HighStruct` _parkourcomponent_2) _parkourcomponent_2))
        (:`Low`
          (set `ParkourComponent.ResultStruct` (`ParkourComponent.LowStruct` _parkourcomponent_2) _parkourcomponent_2))
        (:`Jump`
          (set `ParkourComponent.ResultStruct` (`ParkourComponent.JumpStruct` _parkourcomponent_2) _parkourcomponent_2)))
      (`self.M_Parkour` _outlocation1 _outlocation2 _parkourtype (`ParkourComponent.ResultStruct` (`self.ParkourComponent`)))
      (else
        (`self.Jump`))))
  (:`Released`
    (`self.StopJumping`)))

(event `Parkour_NMC`
  (params (InLocation1 :type "Vector Structure") (InLocation2 :type "Vector Structure"))
  (`MotionWarpingComponent.AddOrUpdateWarpTarget` (`self.MotionWarping`) (make `MotionWarpingTarget` "ParkourPoint1" InLocation1 (`self.K2_GetActorRotation`)))
  (`MotionWarpingComponent.AddOrUpdateWarpTarget` (`self.MotionWarping`) (make `MotionWarpingTarget` "ParkourPoint1" InLocation2 (`self.K2_GetActorRotation`))))

(event `Parkour_Server`
  (params (InLocation1 :type "Vector Structure") (InLocation2 :type "Vector Structure"))
  (`self.Parkour_NMC` InLocation1 InLocation2))

(fn `Parkour Trace BP`
  (params (Initial_Trace_Length :type "Float (double-precision)") (Trace_Z_Offset :type "Float (double-precision)") (Falling_Height_Multiplier :type "Float (double-precision)") (DebugTrace :type "EDrawDebugTrace Enum" :default "None"))
  (returns (InParkourPos1 :type "Vector Structure") (InParkourPso2 :type "Vector Structure"))
  (locals (MantlePos1 :type "Vector Structure") (MantlePos2 :type "Vector Structure"))
  (bind _returnvalue (`self.K2_GetActorLocation`))
  (bind (_mantlepos1_x _mantlepos1_y) (`KismetMathLibrary.BreakVector` (`local.MantlePos1`)))
  (bind _returnvalue_2 (+ (`local.MantlePos2`) (0.0 0.0 100.0)))
  ;[1 1 1] Trace to Check for an Obejct
  (set `self.CanParkour` false)
  (bind (_outhit _returnvalue_3) (`KismetSystemLibrary.LineTraceSingle` :`Start` _returnvalue :`End` (+ _returnvalue (* (`self.GetActorForwardVector`) Initial_Trace_Length)) :`TraceChannel` "TraceTypeQuery1" :`DrawDebugType` (`local.DebugTrace`)))
  ;[1 1 1] Object가 발견되면 Object 높이를 추적합니다. Player가 Falling이면 최대 도달 가능 높이가 낮아집니다
  (if _returnvalue_3
    (bind (_bblockinghit _binitialoverlap _time _distance _location) (`GameplayStatics.BreakHitResult` _outhit))
    (bind (_outhit_2 _returnvalue_4) (`KismetSystemLibrary.SphereTraceSingle` :`Start` (+ _location (`KismetMathLibrary.MakeVector` 0.0 0.0 (* (`local.Trace_Z_Offset`) (`KismetMathLibrary.SelectFloat` (`local.Falling_Height_Multiplier`) 1.0 (`NavMovementComponent.IsFalling` (`self.CharacterMovement`)))))) :`End` _location :`Radius` 10.0 :`TraceChannel` "TraceTypeQuery1" :`DrawDebugType` (`local.DebugTrace`)))
    ;[1 1 1] 추적에서 검출된 점을 사용하여 이동 워프할 위치 찾기
    (if _returnvalue_4
      (bind (_bblockinghit_2 _binitialoverlap_2 _time_2 _distance_2 _location_2 _impactpoint) (`GameplayStatics.BreakHitResult` _outhit_2))
      (set `local.MantlePos1` (+ _impactpoint (* (`self.GetActorForwardVector`) -50.0)))
      (bind _output_get (set `local.MantlePos2` (+ _impactpoint (* (`self.GetActorForwardVector`) 120.0))))
      ;[1 1 1] 이것은 두 번째 모션 워프 위치를 추론합니다.
      (set `self.CanParkour` true)
      (bind _returnvalue_5 (+ _output_get (0.0 0.0 20.0)))
      (bind (_outhit_3 _returnvalue_6) (`KismetSystemLibrary.SphereTraceSingle` :`Start` _returnvalue_5 :`End` _returnvalue_5 :`Radius` 10.0 :`TraceChannel` "TraceTypeQuery1" :`DrawDebugType` (`local.DebugTrace`)))
      (if _returnvalue_6
        (set `self.CanParkour` false)
        (else
          (set `local.MantlePos2` (+ _impactpoint (* (`self.GetActorForwardVector`) 50.0)))))
      ;[1 1 1] 첫 번째와 두 번째 맨틀 위치의 경로가 명확한지 확인하기 위해 마지막 추적을 수행
      (if (or (== (`local.MantlePos1`) (0.0 0.0 0.0)) (== (`local.MantlePos2`) (0.0 0.0 0.0)))
        (set `self.CanParkour` false :!label _label)
        (else
          (bind (_outhit_4 _returnvalue_7) (`KismetSystemLibrary.SphereTraceSingle` :`Start` (`KismetMathLibrary.MakeVector` _mantlepos1_x _mantlepos1_y (.z _returnvalue_2)) :`End` _returnvalue_2 :`Radius` 10.0 :`TraceChannel` "TraceTypeQuery1" :`DrawDebugType` (`local.DebugTrace`)))
          (if _returnvalue_7
            (goto _label)
            (else
              _))))
      (return (`local.MantlePos1`) (`local.MantlePos2`)))
    (else
      (set `self.CanParkour` false))))

(fn `UserConstructionScript`)