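; Push game mode character Blueprint that plays a material appearance effect on the character.
; PlayMaterialEvent calls its NMC counterpart, which restarts a Timeline from the beginning.
; Each Timeline update writes the curve value to the "Appearance" scalar parameter on every material in MyMaterials.
; Tick only calls the parent, and a debug print of the StateComponent's current state is left disconnected.
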(event `self.ReceiveTick`
  (params (DeltaSeconds :type "Float (single-precision)"))
  (`parent.ReceiveTick` DeltaSeconds))

(event `self.PlayMaterialEvent`
  (`self.PlayMaterialEvent_NMC`))

(event `PlayMaterialEvent_NMC`
  (bind (_direction `_새_트랙_0`) (`Timeline|타임라인` :!via `PlayFromStart`)
    (:`Update`
      (`|ExecutionSequence`
        (:`then_0`
          (for _array_element (`self.MyMaterials`)
            (`MaterialInstanceDynamic.SetScalarParameterValue` _array_element "Appearance" `_새_트랙_0`)))))))

(fn `UserConstructionScript`)