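; BP_BombCharacter is the Bomb game type's character Blueprint, handling a material "Appearance" effect.
; PlayMaterialEvent calls an NMC counterpart (likely a net multicast), whose event restarts a timeline.
; Each timeline update writes the track value to the "Appearance" scalar parameter on every MyMaterials entry and the mesh's dynamic overlay material.
; BeginPlay, Tick and the construction script are empty, and a walk-speed debug print is disconnected.
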(event `self.PlayMaterialEvent`
  (`self.PlayMaterialEvent_NMC`))

(event `PlayMaterialEvent_NMC`
  (bind (_direction `_새_트랙_0`) (`Timeline|타임라인` :!via `PlayFromStart`)
    (:`Update`
      (`|ExecutionSequence`
        (:`then_0`
          (for _array_element (`self.MyMaterials`)
            (`MaterialInstanceDynamic.SetScalarParameterValue` _array_element "Appearance" `_새_트랙_0`)))
        (:`then_1`
          (bind `_as머티리얼_인스턴스_다이내믹` (cast `MaterialInstanceDynamic` (`MeshComponent.OverlayMaterial` (`self.Mesh`))))
          (`MaterialInstanceDynamic.SetScalarParameterValue` `_as머티리얼_인스턴스_다이내믹` "Appearance" `_새_트랙_0`))))))

(event `self.ReceiveBeginPlay`)

(event `self.ReceiveTick`
  (params (DeltaSeconds :type "Float (single-precision)")))

(fn `UserConstructionScript`)