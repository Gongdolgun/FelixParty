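; Controller for the Bomb game type that brings up the main Bomb UI when gameplay starts.
; On BeginPlay it binds to the DefaultGameState's game-state-type change event.
; When the new type is GamePlay, the local controller creates WDG_BombMain and adds it to the viewport.
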(event `self.ReceiveBeginPlay`
  (bind _asdefault_game_state (cast `DefaultGameState` (`GameplayStatics.GetGameState`)))
  (add `DefaultGameState.OnGameStateTypeChanged` _asdefault_game_state (delegate `CreateWidgetNMC`)))

(event `CreateWidgetNMC`
  (params (InPrevGameType :type "EGameStateType Enum" :default "Ready") (InNewGameType :type "EGameStateType Enum" :default "Ready"))
  (if (`|EnumEquality` InNewGameType "GamePlay")
    (`self.createWidget`)))

(event `createWidget`
  (if (`self.IsLocalController`)
    (bind _returnvalue (`|CreateWidget` "/Game/GameTypes/Bomb/Widget/WDG_BombMain.WDG_BombMain_C"))
    (`UserWidget.AddToViewport` _returnvalue 0)))

(fn `UserConstructionScript`)