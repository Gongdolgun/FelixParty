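; First-person shooter player controller that manages the local player's crosshair HUD and kill log.
; On BeginPlay it binds to DefaultGameState events for game-state type changes and character deaths.
; Switching to GamePlay creates the crosshair widget on the local controller only, and each death event forwards attacker and victim names to that widget's kill log.
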(event `SomeoneDeadEvent`
  (params (InAttackerName :type String) (InHittedCharacterName :type String))
  (bind _wdg_crosshair (`self.WDG_CrossHair`)
    (:`then`
      (`/Game/Widgets/InGame/WDG_KillLog.AddKillLogEvent` (`/Game/GameTypes/FPS/Widgets/WDG_CrossHair.WDG_KillLog` _wdg_crosshair) InAttackerName InHittedCharacterName))
    (:`else`)))

(event `self.ReceiveBeginPlay`
  (bind _asdefault_game_state (cast `DefaultGameState` (`GameplayStatics.GetGameState`)))
  (add `DefaultGameState.OnGameStateTypeChanged` _asdefault_game_state (delegate `CreateWidgetNMC`))
  (add `DefaultGameState.OnSomeoneDead` _asdefault_game_state (delegate `SomeoneDeadEvent`)))

(event `CreateWidgetNMC`
  (params (InPrevGameType :type "EGameStateType Enum" :default "Ready") (InNewGameType :type "EGameStateType Enum" :default "Ready"))
  (if (`|EnumEquality` InNewGameType "GamePlay")
    (`self.CreateCrosshairWidget`)))

(event `CreateCrosshairWidget`
  (if (`self.IsLocalController`)
    (bind _returnvalue (`|CreateWidget` "/Game/GameTypes/FPS/Widgets/WDG_CrossHair.WDG_CrossHair_C"))
    (`UserWidget.AddToViewport` _returnvalue 0)
    (set `self.WDG_CrossHair` _returnvalue)))

(fn `UserConstructionScript`)