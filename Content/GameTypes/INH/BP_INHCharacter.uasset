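; Character Blueprint for the INH game type that handles material-driven appearance and death effects.
; PlayMaterialEvent and DeadMaterialEvent each forward to an NMC counterpart (likely NetMulticast) that plays its own timeline.
; Each timeline update drives the Appearance scalar on every material in MyMaterials and sets a fixed high Emissive.
; The death timeline destroys the actor when it finishes.
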(event `self.PlayMaterialEvent`
  (`self.PlayMaterialEvent_NMC`))

(event `PlayMaterialEvent_NMC`
  (bind (_direction `_새_트랙_0`) (`Timeline|타임라인` :!via `PlayFromStart`)
    (:`Update`
      (for _array_element (`self.MyMaterials`)
        (`MaterialInstanceDynamic.SetScalarParameterValue` _array_element "Appearance" `_새_트랙_0`)
        (`MaterialInstanceDynamic.SetScalarParameterValue` _array_element "Emissive" 300.0)))))

(event `self.DeadMaterialEvent`
  (`self.DeadMaterialEvent_NMC`))

(event `DeadMaterialEvent_NMC`
  (bind (_direction `_새_트랙_0`) (`Timeline|타임라인_0` :!via `PlayFromStart`)
    (:`Update`
      (for _array_element (`self.MyMaterials`)
        (`MaterialInstanceDynamic.SetScalarParameterValue` _array_element "Appearance" `_새_트랙_0`)
        (`MaterialInstanceDynamic.SetScalarParameterValue` _array_element "Emissive" 300.0)))
    (:`Finished`
      (`self.K2_DestroyActor`))))

(fn `UserConstructionScript`)