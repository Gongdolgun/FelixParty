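; BP_INHController is the controller for the INH game type that manages the local player's main HUD widget.
; On BeginPlay it binds to the INH game state's type-change and death events.
; Entering GamePlay creates WDG_INHMain on the local controller only and adds it to the viewport.
; Death events pass the attacker and victim names on to that widget when it is valid.
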(event `SomeoneDead_Event`
  (params (InAttackerName :type String) (InHittedCharacterName :type String))
  (bind _inhmain (`self.INHMain`)
    (:`then`
      (`INHMain.SomeoneDead` _inhmain InAttackerName InHittedCharacterName))
    (:`else`)))

(event `self.ReceiveBeginPlay`
  (bind _asinhgame_state (cast `INHGameState` (`GameplayStatics.GetGameState`)))
  (add `DefaultGameState.OnGameStateTypeChanged` _asinhgame_state (delegate `CreateWidgetNMC`))
  (add `INHGameState.OnSomeoneDead` _asinhgame_state (delegate `SomeoneDead_Event`)))

(event `CreateWidgetNMC`
  (params (InPrevGameType :type "EGameStateType Enum" :default "Ready") (InNewGameType :type "EGameStateType Enum" :default "Ready"))
  (if (`|EnumEquality` InNewGameType "GamePlay")
    (`self.CreateINHWidget`)))

(event `CreateINHWidget`
  (if (`self.IsLocalController`)
    (bind _returnvalue (`|CreateWidget` "/Game/GameTypes/INH/Widgets/WDG_INHMain.WDG_INHMain_C"))
    (`UserWidget.AddToViewport` _returnvalue 0)
    (set `self.INHMain` _returnvalue)))

(fn `UserConstructionScript`)