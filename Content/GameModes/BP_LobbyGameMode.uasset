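; Lobby game mode that tracks connected lobby controllers and their player info, including name and ready state.
; On post login it records the new controller, naming players by unique net ID and marking the local host ready.
; UpdatePlayerLists rebuilds the info array from all controllers, forcing the host to ready.
; Both paths wait briefly, then push the list to every controller via UpdatePlayerList.
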(event `self.K2_PostLogin`
  (params (NewPlayer :type "PlayerController Object Reference"))
  ;[1 1 1] On Post Login
  (bind _asbp_lobby_controller (cast `/Game/Controllers/BP_LobbyController` NewPlayer))
  (`KismetArrayLibrary.Array_Add` (`self.ConnectedPlayers`) _asbp_lobby_controller)
  (if (`Controller.IsLocalController` _asbp_lobby_controller)
    (bind _returnvalue (`KismetTextLibrary.Conv_StringToText` (`AdvancedSessionsLibrary.UniqueNetIdToString` (`AdvancedSessionsLibrary.GetUniqueNetID` _asbp_lobby_controller))))
    (`KismetArrayLibrary.Array_Add` (`self.ConnectedPlayerInfo`) (make `/Game/Structures/ST_PlayerInfo` _returnvalue true null))
    (else
      (bind _structout (setmembers `/Game/Structures/ST_PlayerInfo` :`StructRef` (`/Game/Controllers/BP_LobbyController.PlayerInfo` _asbp_lobby_controller) :`PlayerName` _returnvalue))
      (`KismetArrayLibrary.Array_Add` (`self.ConnectedPlayerInfo`) _structout)))
  (`KismetSystemLibrary.Delay` 0.2)
  (for _array_element (`self.ConnectedPlayers`)
    (`/Game/Controllers/BP_LobbyController.UpdatePlayerList` _array_element (`self.ConnectedPlayerInfo`))))

(event `UpdatePlayerLists`
  ;[1 1 1] 연결 되어 있는 호스트, 서버 상태 업데이트
  (`KismetArrayLibrary.Array_Clear` (`self.ConnectedPlayerInfo`))
  (for _array_element (`self.ConnectedPlayers`)
    (if (`Controller.IsLocalController` _array_element)
      (bind _output_get (set `/Game/Controllers/BP_LobbyController.PlayerInfo` (make `/Game/Structures/ST_PlayerInfo` (`KismetTextLibrary.Conv_StringToText` (`AdvancedSessionsLibrary.UniqueNetIdToString` (`AdvancedSessionsLibrary.GetUniqueNetID` _array_element))) true null) _array_element))
      (bind _structout (setmembers `/Game/Structures/ST_PlayerInfo` :`StructRef` _output_get :`IsReady` true))
      (`KismetArrayLibrary.Array_Add` (`self.ConnectedPlayerInfo`) _structout)
      (else
        (`KismetArrayLibrary.Array_Add` (`self.ConnectedPlayerInfo`) (`/Game/Controllers/BP_LobbyController.PlayerInfo` _array_element)))))
  (`KismetSystemLibrary.Delay` 0.2)
  (for _array_element_2 (`self.ConnectedPlayers`)
    (`/Game/Controllers/BP_LobbyController.UpdatePlayerList` _array_element_2 (`self.ConnectedPlayerInfo`))))

(fn `UserConstructionScript`)