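; Office file cabinet furniture Blueprint for the level kit that dresses itself with props in the construction script.
; It calls SpawnMeshesFromSockets to scatter desk item meshes into HISMs from "Desk"-prefixed sockets on the furniture mesh.
; A seeded random stream picks a trash can mesh or cube placeholder, weighted toward the can, and jitters its yaw.
; The mesh swap's return value drives that component's visibility and scale.
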(fn `UserConstructionScript`
  (bind _trashcan (`self.TrashCan`))
  (`parent.UserConstructionScript`)
  ;[1 1 1] Spawn Desk Items
  (`self.SpawnMeshesFromSockets` (`self.DeskItemHISMs`) (`self.DeskItemMeshes`) (`self.FurnitureMesh1`) "Desk")
  ;[1 1 1] Handle Trash Can
  (bind _returnvalue (`StaticMeshComponent.SetStaticMesh` _trashcan (select `bool` (`KismetMathLibrary.RandomBoolWithWeightFromStream` (`self.RandomSeedStruct`) 0.8) :`false` "/Engine/BasicShapes/Cube.Cube" :`true` "/Game/Assets/BrutalistLevelKit/Models/Props/Furnitures/SM_Trash_Can.SM_Trash_Can" :!type "StaticMesh Object Reference")))
  (bind _returnvalue_2 (not _returnvalue))
  (`SceneComponent.SetVisibility` _trashcan _returnvalue_2 false)
  (bind _returnvalue_3 (select `bool` _returnvalue_2 :`false` 0.05 :`true` 1.0))
  (`SceneComponent.SetRelativeScale3D` _trashcan (`KismetMathLibrary.MakeVector` _returnvalue_3 _returnvalue_3 _returnvalue_3))
  (`SceneComponent.K2_SetRelativeRotation` _trashcan (`KismetMathLibrary.MakeRotator` 0.0 0.0 (+ (`KismetMathLibrary.RandomFloatInRangeFromStream` (`self.RandomSeedStruct`) -30.0 30.0) 180.0)) false false))